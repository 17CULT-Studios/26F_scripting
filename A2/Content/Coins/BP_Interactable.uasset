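; Data-driven interactable actor whose interaction behavior comes from its DataAsset.
; OnInteract prints the actor's name for debugging, destroys it if the asset flags it, then spawns objects and returns the DataAsset to the caller.
; Spawn class and count come from a nested data asset, when valid, and copies appear above the actor with its rotation and scale.
; Destruction is requested before spawning, and the event graph is unused.
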(fn `OnInteract`
  (params (Player :type "Actor Object Reference"))
  (returns (DataAsset :type "/Game/Coins/PDA_Item Object Reference"))
  (`self.PrintDebugString`)
  (`self.RemoveActorIfNeeded`)
  (`self.SpawnObjects`)
  (return (`self.DataAsset`)))

(fn `PrintDebugString`
  (`KismetSystemLibrary.PrintString` (`KismetStringLibrary.Concat_StrStr` "Interacted with " (`KismetSystemLibrary.GetDisplayName` self))))

(fn `RemoveActorIfNeeded`
  (if (`/Game/Coins/PDA_Item.DestroyOnInteract` (`self.DataAsset`))
    (`self.K2_DestroyActor`)))

(fn `SpawnObjects`
  (bind (_returnvalue_location _returnvalue_rotation _returnvalue_scale) (`KismetMathLibrary.BreakTransform` (`self.GetTransform`)))
  (bind _dataassettospawn (`/Game/Coins/PDA_Item.DataAssetToSpawn` (`self.DataAsset`))
    (:`then`
      (for _ (range 1 (+ (`/Game/Coins/PDA_Item.SpawnAmount` _dataassettospawn) 1))
        (`|SpawnActorFromClass` (`/Game/Coins/PDA_Item.BlueprintType` _dataassettospawn) (`KismetMathLibrary.MakeTransform` (+ _returnvalue_location (0.0 0.0 300.0)) _returnvalue_rotation _returnvalue_scale) "AdjustIfPossibleButAlwaysSpawn" "MultiplyWithRoot" null null)))
    (:`else`)))

(fn `UserConstructionScript`)