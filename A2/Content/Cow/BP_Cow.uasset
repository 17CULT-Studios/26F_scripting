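; BP_Cow is a cow pawn that the player can toggle into or out of following them by interacting with it.
; OnInteract stores the interacting player and flips the Follow flag.
; While Follow is set, Tick reissues AIMoveTo toward the player's current location every frame and clears the IsWalking and IsEating flags.
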(event `self.ReceiveTick`
  (params (DeltaSeconds :type "Float (single-precision)"))
  (if (`self.Follow`)
    (`|AIMoveTo` self (`self.K2_GetActorLocation` (`self.Player`)) null
      (:`then`
        (set `self.bIsWalking` false)
        (set `self.bIsEating` false)))))

(fn `OnInteract`
  (params (Player :type "Actor Object Reference"))
  (returns (DataAsset :type "/Game/Coins/PDA_Item Object Reference"))
  (set `self.Player` Player)
  (set `self.Follow` (not (`self.Follow`)))
  (return null))

(fn `UserConstructionScript`)