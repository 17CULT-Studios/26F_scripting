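; BP_FloatingActor is an actor that spins and bobs in place, like a hovering object.
; BeginPlay stores the starting height, then each Tick adds yaw scaled by RotationSpeed and delta time.
; Tick also sets the Z position to that stored height plus a sine of game time scaled by BobHeight, leaving X and Y unchanged.
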(event `self.ReceiveBeginPlay`
  (bind (_returnvalue_x _returnvalue_y _returnvalue_z) (`KismetMathLibrary.BreakVector` (`self.K2_GetActorLocation`)))
  (set `self.StartingHeight` _returnvalue_z))

(event `self.ReceiveTick`
  (params (DeltaSeconds :type "Float (single-precision)"))
  (bind (_returnvalue_x _returnvalue_y) (`KismetMathLibrary.BreakVector` (`self.K2_GetActorLocation`)))
  (`|ExecutionSequence`
    (:`then_0`
      ; Rotate Object
      (`self.K2_AddActorLocalRotation` (`KismetMathLibrary.MakeRotator` 0.0 0.0 (* DeltaSeconds (`self.RotationSpeed`)))))
    (:`then_1`
      ; Bob Object
      (`self.K2_SetActorLocation` (`KismetMathLibrary.MakeVector` _returnvalue_x _returnvalue_y (+ (`self.StartingHeight`) (* (`KismetMathLibrary.Sin` (`GameplayStatics.GetTimeSeconds`)) (`self.BobHeight`))))))))

(fn `UserConstructionScript`)